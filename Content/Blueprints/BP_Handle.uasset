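; Coffee handle actor that tracks whether it is filled with coffee and works with a machine it references.
; On begin play it turns off collision on its Coffee and Cylinder components and hides the coffee.
; FillCoffee reveals the coffee and sets IsFilled.
; SnapHandle forwards the snap request to the referenced machine, which owns that logic.
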(event Custom|SnapHandle
  (Default|SnapHandle (Variables|Default|GetMachineRef)))

(event Custom|FillCoffee
  (Rendering|SetVisibility (Variables|Default|GetCoffee) true false)
  (Variables|Default|SetisFilled true))

(event EventBeginPlay
  (bind _coffee (Variables|Default|GetCoffee))
  (Collision|SetCollisionEnabled _coffee "NoCollision")
  (Rendering|SetVisibility _coffee false false))

(fn ConstructionScript)