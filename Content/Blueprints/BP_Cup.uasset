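; BP_Cup is a drinkable coffee cup that works with a machine it references.
; Its liquid mesh starts hidden with collision disabled; nothing in this Blueprint makes it visible.
; Drink runs only while the cup is not empty, hiding the liquid, flattening its Z scale, fading in a sip sound and setting IsEmpty.
; SnapHandle forwards to the referenced machine's SnapCup.
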(event Custom|SnapHandle
  (Default|SnapCup (Variables|Default|GetMachineRef)))

(event Custom|Drink
  (bind _liquidmesh (Variables|Default|GetLiquidMesh))
  (bind _returnvalue (Transformation|GetWorldScale _liquidmesh))
  (if (not (Variables|Default|GetisEmpty))
    (Rendering|SetVisibility _liquidmesh false false)
    (Transformation|SetWorldScale3D _liquidmesh (Math|Vector|MakeVector (.x _returnvalue) (.y _returnvalue) 0.0))
    (Audio|Components|Audio|FadeIn (Variables|Default|GetSip_Coffee) 0.05 1.0 0.0 "Linear" :!class /Script/Engine.AudioComponent)
    (Variables|Default|SetisEmpty true)))

(event EventBeginPlay
  (bind _liquidmesh (Variables|Default|GetLiquidMesh))
  (Collision|SetCollisionEnabled _liquidmesh "NoCollision")
  (Rendering|SetVisibility _liquidmesh false false))

(fn ConstructionScript)