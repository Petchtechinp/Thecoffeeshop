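; Coffee machine actor that takes a BP_Handle and BP_Cup and brews a pour on a button press.
; A box overlap tracks both items, and SnapHandle and SnapCup teleport them to their slots with physics off.
; ButtonAnimation runs button timelines; a filled handle starts pour Niagara and audio, and a present cup's liquid scales up by timeline.
; After fixed delays, the pour stops and the handle empties.
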(event OnComponentEndOverlap(Box)
  (params (OverlappedComponent :type Primitive%20Component%20Object%20Reference) (OtherActor :type Actor%20Object%20Reference) (OtherComp :type Primitive%20Component%20Object%20Reference) (OtherBodyIndex :type Integer))
  (if (== (Utilities|GetClass OtherActor) "/Game/Blueprints/BP_Handle.BP_Handle_C")
    (Variables|Default|SetBP%20Handle 0)
    (elif (== (Utilities|GetClass OtherActor) "/Game/Blueprints/BP_Cup.BP_Cup_C")
      (Variables|Default|SetBP%20Cup 0))))

(event OnComponentBeginOverlap(Box)
  (params (OverlappedComponent :type Primitive%20Component%20Object%20Reference) (OtherActor :type Actor%20Object%20Reference) (OtherComp :type Primitive%20Component%20Object%20Reference) (OtherBodyIndex :type Integer) (bFromSweep :type Boolean) (SweepResult :type Hit%20Result%20Structure%20%28by%20ref%29))
  (if (== (Utilities|GetClass OtherActor) "/Game/Blueprints/BP_Handle.BP_Handle_C")
    (bind _asbp_handle (Utilities|Casting|CastToBP_Handle OtherActor))
    (Variables|Default|SetBP%20Handle _asbp_handle)
    (elif (== (Utilities|GetClass OtherActor) "/Game/Blueprints/BP_Cup.BP_Cup_C")
      (bind _asbp_cup (Utilities|Casting|CastToBP_Cup OtherActor))
      (Variables|Default|SetBP%20Cup _asbp_cup))))

(event Custom|ButtonAnimation
  (bind _button (Variables|Default|GetButton))
  (bind _bp_handle (Variables|Default|GetBP%20Handle))
  (bind _bp_cup (Variables|Default|GetBP%20Cup))
  (bind _bp_handle_2 (Variables|Default|GetBP%20Handle))
  (bind _bp_handle_3 (Variables|Default|GetBP%20Handle))
  (bind _liquidmesh (Variables|/Game/Blueprints/BP_Cup.BP_Cup_C|GetLiquidMesh _bp_cup))
  (Variables|Default|SetisAnimated true)
  (if (Utilities|IsValid _bp_handle_3)
    (if (Variables|/Game/Blueprints/BP_Handle.BP_Handle_C|GetisFilled _bp_handle_3)
      (Components|Activation|SetActive (Variables|Default|GetNS_LuqiudPour) true true)
      (Audio|Components|Audio|FadeIn (Variables|Default|GetCoffee_Machine_Pour_Coffee) 0.05 1.0 0.0 "Linear" :!class /Script/Engine.AudioComponent)
      (if (Utilities|IsValid (Variables|Default|GetBP%20Cup))
        (Utilities|FlowControl|Sequence
          (:then_0
            (bind _yoffset (Timeline|ButtonPressed PlayFromStart)
              (:Update
                (Transformation|SetRelativeLocation _button (Math|Vector|MakeVector 0.0 _yoffset 41.444049) false false))
              (:Finished
                (bind _yoffset_2 (Timeline|Timeline ReverseFromEnd)
                  (:Update
                    (Transformation|SetRelativeLocation _button (Math|Vector|MakeVector 0.0 _yoffset_2 41.444049) false false))
                  (:Finished
                    (if (Utilities|IsValid _bp_handle)
                      (if (Variables|/Game/Blueprints/BP_Handle.BP_Handle_C|GetisFilled _bp_handle)
                        (Utilities|FlowControl|Delay 13.0)
                        (Components|Activation|SetActive (Variables|Default|GetNS_LuqiudPour) false false)
                        (Utilities|FlowControl|Delay 2.439728)
                        (Rendering|SetVisibility (Variables|/Game/Blueprints/BP_Handle.BP_Handle_C|GetCoffee _bp_handle_2) false false)
                        (Variables|/Game/Blueprints/BP_Handle.BP_Handle_C|SetisFilled _bp_handle_2 false)
                        (Audio|Components|Audio|FadeOut (Variables|Default|GetCoffee_Machine_Pour_Coffee) 0.05 0.0 "Linear" :!class /Script/Engine.AudioComponent)))
                    (Variables|Default|SetisAnimated false))))))
          (:then_1
            (Rendering|SetVisibility _liquidmesh true false)
            (if (Variables|/Game/Blueprints/BP_Cup.BP_Cup_C|GetisEmpty _bp_cup)
              (bind _zscaleoffset (Timeline|FillCup PlayFromStart)
                (:Update
                  (Transformation|SetWorldScale3D _liquidmesh (Math|Vector|MakeVector 0.827115 0.827115 _zscaleoffset))
                  (Variables|/Game/Blueprints/BP_Cup.BP_Cup_C|SetisEmpty _bp_cup false)))
              (else
                (Timeline|FillCup Play)))))
        (else
          (Timeline|ButtonPressed PlayFromStart)))
      (else
        (Timeline|ButtonPressed PlayFromStart)))
    (else
      (Timeline|ButtonPressed PlayFromStart))))

(event Custom|SnapHandle
  (if (Utilities|IsValid (Variables|Default|GetBP%20Handle))
    (CallFunction|SnapObject (Variables|Default|GetHandlePosition) (Variables|/Game/Blueprints/BP_Handle.BP_Handle_C|GetHandleMesh (Variables|Default|GetBP%20Handle)))))

(event Custom|SnapCup
  (if (Utilities|IsValid (Variables|Default|GetBP%20Cup))
    (CallFunction|SnapObject (Variables|Default|GetCupPosition) (Variables|/Game/Blueprints/BP_Cup.BP_Cup_C|GetCupMesh (Variables|Default|GetBP%20Cup)))))

(event EventBeginPlay
  (Components|Activation|SetActive (Variables|Default|GetNS_LuqiudPour) false false))

(fn ConstructionScript)

(fn SnapObject
  (params (SnapPosition :type Arrow%20Component%20Object%20Reference) (SnapComponent :type Static%20Mesh%20Component%20Object%20Reference))
  (Audio|Components|Audio|FadeIn (Variables|Default|GetPick-Up-Cup) 0.05 1.0 0.0 "Linear" :!class /Script/Engine.AudioComponent)
  (Transformation|SetWorldLocationAndRotation SnapComponent (Transformation|GetWorldLocation SnapPosition) (Transformation|GetWorldRotation SnapPosition) false true)
  (Physics|SetSimulatePhysics SnapComponent false))